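; Cave entrance actor in the PCG level that sends the player into the Dungeons level on interaction.
; Interact stores the PlayerRespawn transform in the PCG game instance and derives a cave seed from the sum of its rounded coordinates, tying the seed to the entrance's position.
; The entrance destroys itself when its ChunkDetector stops overlapping a Chunk, so it disappears along with its terrain.
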(event OnComponentEndOverlap(ChunkDetector)
  (params (OverlappedComponent :type Primitive%20Component%20Object%20Reference) (OtherActor :type Actor%20Object%20Reference) (OtherComp :type Primitive%20Component%20Object%20Reference) (OtherBodyIndex :type Integer))
  (Utilities|Casting|CastToChunk OtherActor)
  (Actor|DestroyActor))

(event EventInteract
  ;[1 1 1] Enter Cave
  (Development|PrintString "Enter")
  (bind _aspcggame_instance (Utilities|Casting|CastToPCGGameInstance (Game|GetGameInstance)))
  (bind _output_get (Variables|/Game/PCGLevel/PCGGameInstance.PCGGameInstance_C|SetPlayerTransform _aspcggame_instance (Transformation|GetWorldTransform (Variables|Default|GetPlayerRespawn))))
  (Variables|/Game/PCGLevel/PCGGameInstance.PCGGameInstance_C|SetCurrentCaveSeed _aspcggame_instance (+ (Math|Float|Round (.x (.location _output_get))) (Math|Float|Round (.y (.location _output_get))) (Math|Float|Round (.z (.location _output_get)))))
  (Game|OpenLevel(byName) "Dungeons"))

(fn ConstructionScript)